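; HTTPTest is a test actor that links the game to a matchmaking service through a SocketIO client.
; On BeginPlay, a multiplayer game mode flagged as server emits a hard-coded "helloserver" message.
; Otherwise it shows the main menu, handing it the socket, and binds "joinserver" by function name.
; That event's handler passes the message string to the multiplayer player controller to connect to the host lobby.
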(event `self.ReceiveBeginPlay`
  (bind _socketioclient (`self.SocketIOClient`))
  (bind _asgame_mode_multiplayer (cast `GameModeMultiplayer` (`GameplayStatics.GetGameMode`))
    (:`then`
      (switch `int` (`GameModeMultiplayer.isServer` _asgame_mode_multiplayer)
        (:`0`
          (bind _returnvalue (`|CreateWidget` "/Game/Blueprints/MainMenu.MainMenu_C" null _socketioclient :!label _label))
          (`UserWidget.AddToViewport` _returnvalue 0)
          (`SocketIOClientComponent.BindEventToFunction` _socketioclient "joinserver" "JoinserverCall" null "/"))
        (:`1`
          (`SocketIOClientComponent.Emit` _socketioclient "helloserver" (`SIOJsonValue.ConstructJsonValueString` "MYNAMENOTJEFF") "/"))))
    (:`CastFailed`
      (goto _label))))

(fn `JoinserverCall`
  (params (Message :type "SIOJsonValue Object Reference"))
  (bind _asplayer_controller_multiplayer (cast `PlayerControllerMultiplayer` (`GameplayStatics.GetPlayerController` 0)))
  (`PlayerControllerMultiplayer.ConnectToHostLobby` _asplayer_controller_multiplayer (`SIOJsonValue.AsString` Message)))

(fn `UserConstructionScript`)